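; BP_collectible is a pickup actor that is drawn into the player and destroyed when BP_Player overlaps it.
; On overlap it prints the other actor's name, then plays the Reduce timeline if the cast to BP_Player succeeds.
; Each update lerps its current location toward the player's live position and its scale toward zero, using separate tracks.
; When the timeline finishes, it calls the OnCollect dispatcher and destroys itself.
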(event Collision|EventActorBeginOverlap
  (params (OtherActor :type Actor%20Object%20Reference))
  (Development|PrintString (Utilities|GetObjectName OtherActor))
  (bind _asbp_player (Utilities|Casting|CastToBP_Player OtherActor))
  (bind (_direction _reduce _move) (Timeline|reduce Play)
    (:Update
      (Transformation|SetActorLocation (Math|Vector|Lerp(Vector) (Transformation|GetActorLocation) (Transformation|GetActorLocation _asbp_player) _move) false false)
      (Transformation|SetActorScale3D (Math|Vector|Lerp(Vector) (Transformation|GetActorScale3D) "0, 0, 0" _reduce)))
    (:Finished
      (Default|CallOnCollect)
      (Actor|DestroyActor))))

(fn ConstructionScript)