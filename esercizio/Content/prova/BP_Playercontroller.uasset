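; Player controller for side-scrolling movement that drives the first player pawn along the Y axis with double jump and dash.
; Tick moves and yaws the pawn when horizontal input passes a deadzone, keeping the last facing.
; Jump and dash use timelines to lerp actor location directly, upward or sideways by facing.
; Boolean flags with post-timeline delays gate re-triggering and the single extra mid-jump.
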(event EventTick
  (params (DeltaSeconds :type Float%20%28single-precision%29))
  (bind _returnvalue (Game|Player|GetPlayerPawn 0))
  (bind _returnvalue_2 (Input|AxisValues|GetMoveRight))
  (bind _rotation (Variables|Default|Getrotation))
  (bind _returnvalue_3 (> _returnvalue_2 0.8))
  (bind _returnvalue_4 (< _returnvalue_2 -0.8))
  (bind _returnvalue_5 (Transformation|GetActorLocation _returnvalue))
  (bind _returnvalue_6 (* _returnvalue_2 _rotation))
  (bind _returnvalue_7 (Math|Rotator|MakeRotator 0.0 0.0 _returnvalue_6))
  (bind _returnvalue_8 (or _returnvalue_4 _returnvalue_3))
  (Transformation|SetActorRotation _returnvalue (Variables|Default|GetCharater%20Direction))
  (Variables|Default|SetMoving _returnvalue_8)
  (if _returnvalue_8
    (Variables|Default|SetCharater%20Direction _returnvalue_7)
    (Transformation|SetActorLocationAndRotation _returnvalue (Math|Vector|MakeVector (.x _returnvalue_5) (+ (* (* _returnvalue_2 DeltaSeconds) (Variables|Default|GetVelocità)) (.y _returnvalue_5)) (.z _returnvalue_5)) _returnvalue_7)))

(event Input|ActionEvents|InputActionJump
  (params (Key :type Key%20Structure :default "None"))
  (bind _returnvalue (Game|Player|GetPlayerPawn 0))
  (bind _returnvalue_2 (Transformation|GetActorLocation _returnvalue))
  (:Pressed
    (if (Variables|Default|Getjumping)
      (Variables|Default|Setjumping false)
      (Variables|Default|SetStartPosition (Math|Vector|MakeVector (.x _returnvalue_2) (.y _returnvalue_2) (.z _returnvalue_2)) :!label _label)
      (Variables|Default|SetfinalPosition (Math|Vector|MakeVector (.x _returnvalue_2) (.y _returnvalue_2) (+ (.z _returnvalue_2) 5e+01)))
      (bind _jump (Timeline|jump PlayFromStart)
        (:Update
          (Transformation|SetActorLocation _returnvalue (Math|Vector|MakeVector (.x _returnvalue_2) (.y _returnvalue_2) (Math|Float|Lerp (.z (Variables|Default|GetStartPosition)) (.z (Variables|Default|GetfinalPosition)) _jump)) false false))
        (:Finished
          (Utilities|FlowControl|Delay 1.0)
          (Variables|Default|Setjumping true)
          (Variables|Default|Setsetdoppio true)))
      (elif (Variables|Default|Getsetdoppio)
        (Variables|Default|Setsetdoppio false)
        (goto _label)))))

(event Input|ActionEvents|InputActionDash
  (params (Key :type Key%20Structure :default "None"))
  (bind _returnvalue (Game|Player|GetPlayerPawn 0))
  (bind _returnvalue_2 (Transformation|GetActorLocation _returnvalue))
  (:Pressed
    (if (Variables|Default|Getdashing)
      (Variables|Default|Setdashing false)
      (if (Math|Rotator|Equal(Rotator) (Variables|Default|GetCharater%20Direction) "0,90.000000, 0" 0.0001)
        (Variables|Default|SetfinalPosition (Math|Vector|MakeVector (.x _returnvalue_2) (+ (.y _returnvalue_2) 1.5e+02) (.z _returnvalue_2)))
        (else
          (Variables|Default|SetfinalPosition (Math|Vector|MakeVector 0.0 (+ (.y _returnvalue_2) -1.5e+02) 0.0))))
      (Variables|Default|SetStartPosition (Math|Vector|MakeVector (.x _returnvalue_2) (.y _returnvalue_2) (.z _returnvalue_2)))
      (bind _dash (Timeline|dash PlayFromStart)
        (:Update
          (Transformation|SetActorLocation _returnvalue (Math|Vector|MakeVector (.x _returnvalue_2) (Math|Float|Lerp (.y (Variables|Default|GetStartPosition)) (.y (Variables|Default|GetfinalPosition)) _dash) (.z _returnvalue_2)) false false))
        (:Finished
          (Utilities|FlowControl|Delay 0.3)
          (Variables|Default|Setdashing true))))))

(fn ConstructionScript)